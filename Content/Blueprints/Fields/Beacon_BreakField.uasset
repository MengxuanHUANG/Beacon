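; Field System actor that applies breaking strain to Chaos destructibles within a spherical area.
; On BeginPlay it adds a persistent External Cluster Strain field from a radial falloff node with no falloff, so strain is uniform.
; The Sphere component sets the center, and its world X scale times a multiplier sets the radius.
; A delayed self-destroy chain is unconnected, so the graph never removes the actor.
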(event EventBeginPlay
  (bind _sphere (Variables|Default|GetSphere))
  (Utilities|FlowControl|Sequence
    (:then_0
      (Class|FieldSystemComponent|AddPersistentField (Variables|Field|GetFieldSystemComponent) true "Field_ExternalClusterStrain" 0 (Field|SetRadialFalloff (Variables|Default|GetRadialFalloff) (Variables|Default|GetStrainMagnitude) 0.0 1.0 0.0 (* (.X (Math|Vector|BreakVector (Transformation|GetWorldScale _sphere))) (Variables|Default|Getvar_1)) (Transformation|GetWorldLocation _sphere) "Field_FallOff_None")))))

(event Collision|EventActorBeginOverlap
  (params (OtherActor :type Actor%20Object%20Reference)))

(event EventTick
  (params (DeltaSeconds :type Float%20%28single-precision%29)))

(fn ConstructionScript)