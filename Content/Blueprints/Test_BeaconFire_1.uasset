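; Test beacon fire Blueprint that builds up a particle and sound fire effect over time.
; Activates its particle on BeginPlay, then raises the spark and smoke parameters every Tick without a cap.
; A "Start Flame" burning event sets a flag that makes Tick also raise fire and embers and slowly fade in the audio volume.
; EndBurning deactivates the particle and pauses the audio, leaving the flag set.
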(event Custom|F_BurningEvents_Event_0
  (params (EventName :type String))
  (switch string EventName
    (:StartFlame
      (CallFunction|StartBurn))))

(event EventBeginPlay
  (EventDispatchers|AssignFBurningEvents (delegate Custom|F_BurningEvents_Event_0))
  (Components|Activation|Activate (Variables|Default|Getm_Particle) false))

(event EventTick
  (params (DeltaSeconds :type Float%20%28single-precision%29))
  (bind _m_particle (Variables|Default|Getm_Particle))
  (bind _m_audiocomponent (Variables|Default|Getm_AudioComponent))
  (bind _m_audiocomponent_2 (Variables|Default|Getm_AudioComponent))
  (bind _volumemultiplier (Variables|/Script/Engine.AudioComponent|GetVolumeMultiplier _m_audiocomponent_2))
  (bind _returnvalue (+ _volumemultiplier 0.0005))
  (Variables|Default|SetSparkEffect (+ (Variables|Default|GetSparkEffect) 0.01))
  (Effects|Components|ParticleSystem|SetFloatParameter _m_particle "SparkEffect" (Variables|Default|GetSparkEffect))
  (Variables|Default|SetSmokeEffect (+ (Variables|Default|GetSmokeEffect) 0.01))
  (Effects|Components|ParticleSystem|SetFloatParameter _m_particle "SmokeEffect" (Variables|Default|GetSmokeEffect))
  (if (Variables|Default|GetIsStartBurn)
    (if (not (Audio|Components|Audio|IsPlaying _m_audiocomponent))
      (Audio|Components|Audio|Play _m_audiocomponent 0.0)
      (Audio|Components|Audio|SetVolumeMultiplier _m_audiocomponent_2 0.01 :!class /Script/Engine.AudioComponent)
      (elif (Variables|Default|GetIsStartBurn)
        (if (<= _returnvalue 1.0)
          (Audio|Components|Audio|SetVolumeMultiplier _m_audiocomponent_2 _returnvalue :!class /Script/Engine.AudioComponent))))
    (Variables|Default|SetFireEffect (+ (Variables|Default|GetFireEffect) 0.01))
    (Effects|Components|ParticleSystem|SetFloatParameter _m_particle "FireEffect" (Variables|Default|GetFireEffect))
    (Variables|Default|SetEmbers%20Effect (+ (Variables|Default|GetEmbers%20Effect) 0.01))
    (Effects|Components|ParticleSystem|SetFloatParameter _m_particle "EmbersEffect" (Variables|Default|GetEmbers%20Effect))))

(event EventEndBurning
  (CallFunction|ENd))

(fn StartBurn
  (Variables|Default|SetIsStartBurn true))

(fn ENd
  (Components|Activation|SetActive (Variables|Default|Getm_Particle) false false)
  (Class|AudioComponent|SetPaused (Variables|Default|Getm_AudioComponent) true))