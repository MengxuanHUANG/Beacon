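; Wood fire Blueprint for a beacon fire that drives a particle system and looping states of flame, smoke, embers and audio.
; A "Start Flame" burning event starts smoke and sound, while UpdateFlame maps flame strength to flame parameters and volume.
; Tick calls a custom dispatcher, letting state changes bind and unbind per-frame updates.
; EndFlame zeroes the effects and pauses audio, and DecreaseSmoke2 steps down secondary smoke before unbinding.
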(event Custom|F_BurningEvents_Event
  (params (EventName :type String))
  (switch string EventName
    (:StartFlame
      (CallFunction|StartFlame))))

(event Custom|MyEventDispather_Event
  (params (DeltaTime :type Float%20%28single-precision%29)))

(event EventBeginPlay
  (EventDispatchers|BindEventtoFBurningEvents (delegate Custom|F_BurningEvents_Event)))

(event EventTick
  (params (DeltaSeconds :type Float%20%28single-precision%29))
  (Default|CallMyEventDispather DeltaSeconds))

(event EventStartBurning
  (bind _m_particle (Variables|Default|Getm_Particle))
  (EventDispatchers|UnbindallEventsfromMyEventDispather)
  (Components|Activation|SetActive _m_particle true false)
  (Effects|Components|ParticleSystem|SetFloatParameter _m_particle "Smoke_1" (Variables|Default|GetSmoke_1))
  (Effects|Components|ParticleSystem|SetFloatParameter _m_particle "Ember" (Variables|Default|GetEmber))
  (Effects|Components|ParticleSystem|SetFloatParameter _m_particle "Spark" (Variables|Default|GetSpark))
  (Effects|Components|ParticleSystem|SetFloatParameter _m_particle "Distortion" (Variables|Default|GetDistortion)))

(event EventEndBurning)

(event EventEndFlame
  (bind _m_particle (Variables|Default|Getm_Particle))
  (Variables|Default|SetbHasFlame false)
  (Effects|Components|ParticleSystem|SetFloatParameter _m_particle "Smoke_1" 0.0)
  (Effects|Components|ParticleSystem|SetFloatParameter _m_particle "Ember" 0.0)
  (Effects|Components|ParticleSystem|SetFloatParameter _m_particle "Spark" 0.0)
  (Effects|Components|ParticleSystem|SetFloatParameter _m_particle "Distortion" 0.0)
  (EventDispatchers|BindEventtoMyEventDispather (EventDispatchers|CreateEvent :!event DecreaseSmoke2))
  (Effects|Components|ParticleSystem|SetFloatParameter _m_particle "Flame_1" 0.0)
  (Effects|Components|ParticleSystem|SetFloatParameter _m_particle "Flame_2" 0.0)
  (EventDispatchers|UnbindEventfromMyEventDispather (EventDispatchers|CreateEvent :!event UpdateFlame))
  (Class|AudioComponent|SetPaused (Variables|Default|Getm_AudioComponent) true))

(fn StartFlame
  (Variables|Default|SetbHasFlame true)
  (EventDispatchers|BindEventtoMyEventDispather (EventDispatchers|CreateEvent :!event UpdateFlame))
  (Effects|Components|ParticleSystem|SetFloatParameter (Variables|Default|Getm_Particle) "Smoke_1" (Variables|Default|GetSmoke_1))
  (Audio|Components|Audio|Play (Variables|Default|Getm_AudioComponent) 0.0))

(fn UpdateFlame
  (params (DeltaTime :type Float%20%28single-precision%29))
  (bind _m_particle (Variables|Default|Getm_Particle))
  (bind _m_flamestrength (Variables|Default|Getm_FlameStrength))
  (bind _flame (Utilities|MapStrengthFlame _m_flamestrength))
  (Effects|Components|ParticleSystem|SetFloatParameter _m_particle "Flame_1" _flame)
  (Effects|Components|ParticleSystem|SetFloatParameter _m_particle "Flame_2" _flame)
  (Audio|Components|Audio|SetVolumeMultiplier (Variables|Default|Getm_AudioComponent) (Utilities|MapStrengthAudio _m_flamestrength) :!class /Script/Engine.AudioComponent))

(fn DecreaseSmoke2
  (params (NewParam :type Float%20%28single-precision%29))
  (bind _output_get (Variables|Default|SetSmoke_2 (+ (Variables|Default|GetSmoke_2) -0.002)))
  (if (< (+ (Variables|Default|GetSmoke_2) -0.002) 0.0)
    (EventDispatchers|UnbindEventfromMyEventDispather (EventDispatchers|CreateEvent :!event DecreaseSmoke2))
    (else
      (Effects|Components|ParticleSystem|SetFloatParameter (Variables|Default|Getm_Particle) "Smoke_2" _output_get))))