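; BeaconFire is a beacon fire effect that ignites when a bound burning event fires.
; BeginPlay binds the event handler, whose matching case calls StartBurn to set the burn flag.
; Tick steadily raises spark and smoke particle parameters from the start, adding fire, embers and looping-checked audio playback once burning.
; The ramps use fixed per-frame increments with no delta-time scaling or upper limit.
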(event Custom|F_BurningEvents_Event_0
  (params (EventName :type String))
  (switch string EventName
    (:Case_0
      (CallFunction|StartBurn))))

(event EventBeginPlay
  (EventDispatchers|AssignFBurningEvents (delegate Custom|F_BurningEvents_Event_0)))

(event EventTick
  (params (DeltaSeconds :type Float%20%28single-precision%29))
  (bind _m_particle (Variables|Default|Getm_Particle))
  (bind _m_audiocomponent (Variables|Default|Getm_AudioComponent))
  (Variables|Default|SetSparkEffect (+ (Variables|Default|GetSparkEffect) 0.01))
  (Effects|Components|ParticleSystem|SetFloatParameter _m_particle "SparkEffect" (Variables|Default|GetSparkEffect))
  (Variables|Default|SetSmokeEffect (+ (Variables|Default|GetSmokeEffect) 0.01))
  (Effects|Components|ParticleSystem|SetFloatParameter _m_particle "SmokeEffect" (Variables|Default|GetSmokeEffect))
  (if (Variables|Default|GetIsStartBurn)
    (if (not (Audio|Components|Audio|IsPlaying _m_audiocomponent))
      (Audio|Components|Audio|Play _m_audiocomponent 0.0))
    (Variables|Default|SetFireEffect (+ (Variables|Default|GetFireEffect) 0.01))
    (Effects|Components|ParticleSystem|SetFloatParameter _m_particle "FireEffect" (Variables|Default|GetFireEffect))
    (Variables|Default|SetEmbers%20Effect (+ (Variables|Default|GetEmbers%20Effect) 0.01))
    (Effects|Components|ParticleSystem|SetFloatParameter _m_particle "EmbersEffect" (Variables|Default|GetEmbers%20Effect))))

(fn StartBurn
  (Variables|Default|SetIsStartBurn true))